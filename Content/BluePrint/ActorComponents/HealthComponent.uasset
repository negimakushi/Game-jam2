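; Actor component that tracks an actor's health and gives it an on-screen health bar.
; On BeginPlay it adds a screen-space, collision-free widget component to the owner and fills it with a HealthBar widget initialized with Health and the owning actor.
; TakeDamege subtracts from Health without clamping, fires OnDamageTaken, then fires OnDeath whenever the result is zero or below.
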(event `self.ReceiveBeginPlay`
  (bind _returnvalue (`self.GetOwner`))
  (bind _returnvalue_2 (`|AddComponentByClass` _returnvalue "/Script/UMG.WidgetComponent" false (`KismetMathLibrary.MakeTransform` (100.0 0.0 0.0))))
  (`WidgetComponent.SetDrawSize` _returnvalue_2 (150.0 10.0))
  (`WidgetComponent.SetWidgetSpace` _returnvalue_2 "Screen")
  (`PrimitiveComponent.SetCollisionEnabled` _returnvalue_2 "NoCollision")
  (bind _returnvalue_3 (`|CreateWidget` "/Game/UI/HealthBar.HealthBar_C" null (`self.Health`) _returnvalue))
  (`WidgetComponent.SetWidget` _returnvalue_2 _returnvalue_3))

(fn `TakeDamege`
  (params (Amount :type "Float (double-precision)"))
  (bind _output_get (set `self.Health` (- (`self.Health`) Amount)))
  (`self.OnDamageTaken`)
  (if (<= _output_get 0.0)
    (`self.OnDeath`)))