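; BP_RoamingObject is an item actor that wanders horizontally and destroys itself when its mesh hits the player.
; On BeginPlay it picks a random XY direction, which is not normalized, so effective speed varies with each pick.
; Tick moves it along that direction by Speed with a swept move.
; A mesh hit on anything other than BP_Player generates a new random direction, so it bounces around obstacles.
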(event `self.ReceiveBeginPlay`
  (`self.GenerateDirection`))

(event `self.ReceiveActorBeginOverlap`
  (params (OtherActor :type "Actor Object Reference")))

(event `self.ReceiveTick`
  (params (DeltaSeconds :type "Float (single-precision)"))
  (`self.K2_SetActorLocation` (+ (* DeltaSeconds (`self.Speed`) (`self.Direction`)) (`self.K2_GetActorLocation`)) true))

(event `self.StaticMesh.OnComponentHit`
  (params (HitComponent :type "PrimitiveComponent Object Reference") (OtherActor :type "Actor Object Reference") (OtherComp :type "PrimitiveComponent Object Reference") (NormalImpulse :type "Vector Structure") (Hit :type "HitResult Structure (by ref)"))
  (cast `/Game/BluePrint/Player/BP_Player` OtherActor
    (:`then`
      (`self.K2_DestroyActor`))
    (:`CastFailed`
      (`self.GenerateDirection`))))

(fn `GenerateDirection`
  (set `self.Direction` (`KismetMathLibrary.MakeVector` (`KismetMathLibrary.RandomFloatInRange` -1.0 1.0) (`KismetMathLibrary.RandomFloatInRange` -1.0 1.0))))

(fn `UserConstructionScript`)