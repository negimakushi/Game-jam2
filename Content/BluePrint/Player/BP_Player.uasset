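; BP_Player is the player actor, handling Enhanced Input world-axis movement and an orbiting ring of projectile shooters.
; Space triggers a one-time spawn of BP_Player_Shooter actors evenly around a circle, attached to SpringArmShooter, which rotates every tick.
; Z raises the fire frequency and pushes it to every stored shooter through UpdateShooter, whose Speed input is unused.
; X applies test damage to HealthComponent, whose damage event prints current health.
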(event `self.ReceiveBeginPlay`
  (bind _asplayer_controller (cast `PlayerController` (`self.GetController`)))
  (bind _returnvalue (pcsubsystem `EnhancedInputLocalPlayerSubsystem` _asplayer_controller))
  (`/Engine/EditorBlueprintResources/StandardMacros.IsValid` _returnvalue
    (:`Is Valid`
      (`EnhancedInputSubsystemInterface.AddMappingContext` _returnvalue "/Game/Input/Control.Control" 0 (struct)))))

(event `EnhancedInput|/Game/Input/Move`
  (params (ActionValue :type "Vector2D Structure") (ElapsedSeconds :type "Float (double-precision)") (TriggeredSeconds :type "Float (double-precision)") (InputAction :type "InputAction Object Reference" :default "/Game/Input/Move.Move"))
  (:`Triggered`
    (`self.AddMovementInput` (1.0 0.0 0.0) ActionValue_X)
    (`self.AddMovementInput` (0.0 1.0 0.0) ActionValue_Y)))

(event `Key|X`
  (params (Key :type "Key Structure"))
  (:`Pressed`
    (`/Game/BluePrint/ActorComponents/HealthComponent.TakeDamege` (`self.HealthComponent`) 20.0)))

(event `self.HealthComponent.OnDamageTaken`
  (`KismetSystemLibrary.PrintString` (`KismetStringLibrary.Conv_DoubleToString` (`/Game/BluePrint/ActorComponents/HealthComponent.Health` (`self.HealthComponent`)))))

(event `Key|SpaceBar`
  (params (Key :type "Key Structure"))
  (:`Pressed`
    (`/Engine/EditorBlueprintResources/StandardMacros.DoOnce` false
      (:`Completed`
        (`self.SummonShooter` (`self.K2_GetActorLocation`) (`self.ShooterRadius`) (`self.ShooterNumber`))))))

(event `Key|Z`
  (params (Key :type "Key Structure"))
  (:`Pressed`
    (bind _output_get (set `self.ShooterFrequency` (+ (`self.ShooterFrequency`) 1.0)))
    (`self.UpdateShooter` _output_get)))

(event `self.ReceiveTick`
  (params (DeltaSeconds :type "Float (single-precision)"))
  (`SceneComponent.K2_AddLocalRotation` (`self.SpringArm_Shooter`) (`KismetMathLibrary.MakeRotator` 0.0 0.0 (`self.ShooterRotateSpeed`)) false false))

(fn `SummonShooter`
  (params (Center :type "Vector Structure") (Radius :type "Float (double-precision)") (ObjectNumber :type Integer))
  (bind (_center_x _center_y _center_z) (`KismetMathLibrary.BreakVector` (`local.Center`)))
  (bind _center_x_2 (`KismetMathLibrary.BreakVector` (`local.Center`)))
  (bind (_center_x_3 _center_y_2) (`KismetMathLibrary.BreakVector` (`local.Center`)))
  (set `self.ShooterAngle` (/ (* (`KismetMathLibrary.GetPI`) 2.0) (`local.ObjectNumber`)))
  (for _index (range (`local.ObjectNumber`))
    (bind _returnvalue (`|SpawnActorFromClass` "/Game/BluePrint/Player/BP_Player_Shooter.BP_Player_Shooter_C" (`KismetMathLibrary.MakeTransform` (`KismetMathLibrary.MakeVector` (+ _center_x_2 (* (`local.Radius`) (`KismetMathLibrary.Cos` (* (`self.ShooterAngle`) _index)))) (+ _center_y_2 (* (`local.Radius`) (`KismetMathLibrary.Sin` (* (`self.ShooterAngle`) _index)))) _center_z)) "Undefined" "MultiplyWithRoot" null "/Game/BluePrint/Projectiles/BP_Projectile_Bullet.BP_Projectile_Bullet_C" (`self.ShooterFrequency`) (struct) null))
    (`KismetArrayLibrary.Array_Add` (`self.Shooters`) _returnvalue)
    (`self.K2_AttachToComponent` _returnvalue (`self.SpringArm_Shooter`) "None" "KeepWorld" "KeepWorld" "KeepWorld" true)))

(fn `UpdateShooter`
  (params (Frequency :type "Float (double-precision)") (Speed :type Integer))
  (for _array_element (`self.Shooters`)
    (if (not (<= Frequency 0.0))
      (`/Game/BluePrint/Player/BP_Shooter.UpdateFrequency` _array_element (`self.ShooterFrequency`)))))

(fn `UserConstructionScript`)