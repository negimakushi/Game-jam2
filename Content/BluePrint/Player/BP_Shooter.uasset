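; BP_Shooter is a player-side Blueprint that automatically fires projectiles on a repeating timer.
; BeginPlay starts a looping timer at Frequency seconds, stores its handle, and each tick of it spawns ProjectileType at ShootPoint's transform with BulletSpeed.
; UpdateFrequency clears the stored timer and starts a looping one at the new interval, but does not save the new handle in FrequencyTimer.
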(event `self.ReceiveBeginPlay`
  (bind _returnvalue (`KismetSystemLibrary.K2_SetTimerDelegate` (delegate `Shoot`) (`self.Frequency`) true))
  (set `self.FrequencyTimer` _returnvalue))

(event `Shoot`
  (`|SpawnActorFromClass` (`self.ProjectileType`) (`SceneComponent.K2_GetComponentToWorld` (`self.ShootPoint`)) "Undefined" "MultiplyWithRoot" self (`self.BulletSpeed`) 0.0 null false true null))

(fn `UpdateFrequency`
  (params (NewParam :type "Float (double-precision)"))
  (`KismetSystemLibrary.K2_ClearAndInvalidateTimerHandle` (`self.FrequencyTimer`))
  (`KismetSystemLibrary.K2_SetTimerDelegate` (`|CreateDelegate` :!event `Shoot`) NewParam true))

(fn `UserConstructionScript`)