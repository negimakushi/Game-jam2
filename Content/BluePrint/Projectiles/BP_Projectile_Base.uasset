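; Base projectile actor for player and enemy shots, choosing its collision profile by side and ignoring its owner when moving.
; The construction script feeds speed and gravity into ProjectileMovement and enables homing on a valid target when flagged.
; On BeginPlay it aims its velocity at any valid target.
; On hit it fires a hit callback, plays impact effect and sound except against walls, then destroys itself.
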(event `self.ReceiveBeginPlay`
  (`PrimitiveComponent.IgnoreActorWhenMoving` (`self.Box`) (`self.GetOwner`) true)
  (if (`self.IsPlayerSide`)
    (`PrimitiveComponent.SetCollisionProfileName` (`self.Box`) "PlayerPreSet" true)
    (else
      (`PrimitiveComponent.SetCollisionProfileName` (`self.Box`) "EnemyPreSet" true)))
  (`self.Target`
    (:`then`
      (`self.Rotate to Enemy`))
    (:`else`)))

(event `Rotate to Enemy`
  (set `MovementComponent.Velocity` (* (`KismetMathLibrary.GetDirectionUnitVector` (`self.K2_GetActorLocation`) (`self.K2_GetActorLocation` (`self.Target`))) (`self.Speed`)) (`self.ProjectileMovement`)))

(event `self.Box.OnComponentHit`
  (params (HitComponent :type "PrimitiveComponent Object Reference") (OtherActor :type "Actor Object Reference") (OtherComp :type "PrimitiveComponent Object Reference") (NormalImpulse :type "Vector Structure") (Hit :type "HitResult Structure (by ref)"))
  (bind (_bblockinghit _binitialoverlap _time _distance _location) (`GameplayStatics.BreakHitResult` Hit))
  (`self.OnProjectileHit` OtherActor Hit)
  (cast `/Game/BluePrint/Stage/BP_Wall` OtherActor
    (:`then`
      (`self.K2_DestroyActor`))
    (:`CastFailed`
      (bind _returnvalue (`GameplayStatics.SpawnEmitterAtLocation` (`self.Impact Effect`) _location))
      (`ParticleSystemComponent.EndTrails` _returnvalue)
      (`GameplayStatics.PlaySoundAtLocation` (`self.Impact Sound`) _location (struct) 1.0 1.0 0.0 null null null null)
      (`self.K2_DestroyActor`))))

(fn `UserConstructionScript`
  (bind _projectilemovement (`self.ProjectileMovement`))
  (set `ProjectileMovementComponent.InitialSpeed` (`self.Speed`) _projectilemovement)
  (set `ProjectileMovementComponent.MaxSpeed` (`self.Speed`) _projectilemovement)
  (set `ProjectileMovementComponent.ProjectileGravityScale` (`self.Gravity`) _projectilemovement)
  (`self.Target`
    (:`then`
      (if (`self.Is Homing`)
        (set `ProjectileMovementComponent.bIsHomingProjectile` true _projectilemovement)
        (set `ProjectileMovementComponent.HomingTargetComponent` (`Actor.RootComponent` (`self.Target`)) _projectilemovement)))
    (:`else`)))